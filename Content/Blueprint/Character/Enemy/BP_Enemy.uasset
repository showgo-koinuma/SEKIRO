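; Base enemy character for Sekiro-style posture combat, built on GAS with guarding, parries and deathblows.
; Weapon overlaps deal hit-limited attacks; incoming hits in Normal state trigger guard with half posture impact, otherwise full damage, via SetByCaller effects.
; Parries rewind the montage and drain posture; broken posture shows a deathblow prompt, and TakenDeathblow positions the enemy for front execution.
; Tick faces the player and refreshes posture and lock-on widgets; DisableEnemy ragdolls the body.
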(event `self.ReceiveBeginPlay`
  (`self.SetCollisionReference`)
  (`CharacterParameter.ApplyStatus` (`self.CharacterParameter`) (`self.AbilitySystemComponent`))
  (`self.InitializeWidget`)
  (`AbilitySystemComponent.BP_ApplyGameplayEffectToSelf` :`self` (`self.AbilitySystemComponent`) :`GameplayEffectClass` "/Game/Blueprint/GAS/GE/GE_PostureRegene.GE_PostureRegene_C"))

(event `self.ReceiveTick`
  (params (DeltaSeconds :type "Float (single-precision)"))
  (`self.SetRotationToPlayer` DeltaSeconds)
  (`self.ApplyPostureToWidget`)
  (`self.SetUIVisible`))

(event `self.WeaponCollision.OnComponentBeginOverlap`
  (params (OverlappedComponent :type "PrimitiveComponent Object Reference") (OtherActor :type "Actor Object Reference") (OtherComp :type "PrimitiveComponent Object Reference") (OtherBodyIndex :type Integer) (bFromSweep :type Boolean) (SweepResult :type "HitResult Structure (by ref)"))
  (bind _currentattackhitcount (`self.CurrentAttackHitCount`))
  ;[1 0.3229 0.3229 0.571] 攻撃処理
  (bind _ascharacter_base (cast `CharacterBase` OtherActor))
  (if (> _currentattackhitcount 0)
    (set `self.CurrentAttackHitCount` (- _currentattackhitcount 1))
    (`self.HitAttack` _ascharacter_base (`self.CharacterAttackParam`) (0.0 0.0 0.0) (0.0 0.0 0.0) self)))

(event `ParriedPlayMontage`
  (`|PlayMontage` (`self.Mesh`) (`self.GetCurrentMontage`) -0.5 0.4))

(event `self.OnBrokePosture`
  ;[1 1 1] 体幹が崩れたとき
  (`parent.OnBrokePosture`)
  (`AbilitySystemComponent.TryActivateAbilityByClass` (`self.AbilitySystemComponent`) "/Game/Blueprint/GAS/Enemy/GA_BrokePosture.GA_BrokePosture_C" true))

(event `self.OnDead`
  (`parent.OnDead`)
  (if (`|EnumInequality` (`self.CharacterState`) "Dead")
    (`self.StopAnimMontage` (`self.GetCurrentMontage`))))

(event `self.ApplyHitGameplayEffect`
  (params (Damage :type "Float (single-precision)") (Impact :type "Float (single-precision)"))
  (bind _returnvalue (`AbilitySystemBlueprintLibrary.AssignTagSetByCallerMagnitude` (`AbilitySystemComponent.MakeOutgoingSpec` :`self` (`self.AbilitySystemComponent`) :`GameplayEffectClass` "/Game/Blueprint/GAS/GE/GE_StatusEffect.GE_StatusEffect_C") (struct :`TagName` "Data.Status.CurrentHp") (* Damage -1.0)))
  (bind _returnvalue_2 (`AbilitySystemBlueprintLibrary.AssignTagSetByCallerMagnitude` _returnvalue (struct :`TagName` "Data.Status.Posture.PosturePoint") (* Impact -1.0)))
  (`AbilitySystemComponent.BP_ApplyGameplayEffectSpecToSelf` (`self.AbilitySystemComponent`) _returnvalue_2))

(event `self.ApplyPostureEffect`
  (params (AddValue :type "Float (single-precision)"))
  (bind _returnvalue (`AbilitySystemBlueprintLibrary.AssignTagSetByCallerMagnitude` (`AbilitySystemComponent.MakeOutgoingSpec` :`self` (`self.AbilitySystemComponent`) :`GameplayEffectClass` "/Game/Blueprint/GAS/GE/GE_PostureEffect.GE_PostureEffect_C") (struct :`TagName` "Data.Status.Posture.PosturePoint") AddValue))
  (`AbilitySystemComponent.BP_ApplyGameplayEffectSpecToSelf` (`self.AbilitySystemComponent`) _returnvalue))

(fn `ApplyHpToWidgetOnChanged`
  (bind (_hp_basevalue _hp_currentvalue) (break `GameplayAttributeData` (`CharacterAttributeSet.Hp` (`self.CharacterAttributeSet`))))
  (`/Game/Blueprint/Character/WBP_CharacterUIBase.ChangeHp` (`self.EnemyWidget`) _hp_currentvalue))

(fn `ApplyPostureToWidget`
  (bind (_posturepoint_basevalue _posturepoint_currentvalue) (break `GameplayAttributeData` (`CharacterAttributeSet.PosturePoint` (`self.CharacterAttributeSet`))))
  (set `/Game/Blueprint/Character/WBP_CharacterUIBase.CurrentPosture` _posturepoint_currentvalue (`self.EnemyWidget`)))

(fn `DisableEnemy`
  (bind _mesh (`self.Mesh`))
  (`PrimitiveComponent.SetCollisionEnabled` (`self.CapsuleComponent`) "NoCollision")
  (`PrimitiveComponent.SetCollisionProfileName` _mesh "Ragdoll" true)
  (`PrimitiveComponent.SetSimulatePhysics` _mesh true)
  (`Widget.SetVisibility` (`self.EnemyWidget`) "Hidden"))

(fn `HitAttack`
  (params (AttackParam :type "CharacterAttackParam Object Reference") (Direction :type "Vector Structure") (HitPoint :type "Vector Structure") (Attacker :type "CharacterBase Object Reference"))
  (bind _abilitysystemcomponent (`self.AbilitySystemComponent`))
  (bind _impact (`CharacterAttackParam.Impact` AttackParam))
  (if (`KismetSystemLibrary.IsValid` AttackParam)
    (if (`|EnumEquality` (`self.CharacterState`) "Normal")
      (`self.ApplyHitGameplayEffect` 0.0 (* _impact 0.5))
      (`AbilitySystemComponent.TryActivateAbilityByClass` _abilitysystemcomponent "/Game/Blueprint/GAS/GA/Hit/GA_Gaurd.GA_Gaurd_C" true)
      (`self.ApplyHpToWidgetOnChanged`)
      (else
        (`AbilitySystemComponent.TryActivateAbilityByClass` _abilitysystemcomponent "/Game/Blueprint/GAS/GA/Hit/GA_HitAttack.GA_HitAttack_C" true)
        (`self.ApplyHitGameplayEffect` (`CharacterAttackParam.Damage` AttackParam) _impact)
        (`self.ApplyHpToWidgetOnChanged`)
        (return)))))

(fn `InitializeWidget`
  (bind _characterattributeset (`self.CharacterAttributeSet`))
  (bind (_maxhp_basevalue _maxhp_currentvalue) (break `GameplayAttributeData` (`CharacterAttributeSet.MaxHp` _characterattributeset)))
  (bind (_maxposturepoint_basevalue _maxposturepoint_currentvalue) (break `GameplayAttributeData` (`CharacterAttributeSet.MaxPosturePoint` _characterattributeset)))
  (`|ExecutionSequence`
    (:`then_0`
      ;[1 1 1] デフォルトUI
      (bind _aswbp_enemy_ui (cast `/Game/Blueprint/Character/Enemy/WBP_EnemyUI` (`WidgetComponent.GetWidget` (`self.EnemyUI`))))
      (bind _output_get (set `self.EnemyWidget` _aswbp_enemy_ui))
      (set `/Game/Blueprint/Character/WBP_CharacterUIBase.MaxHp` _maxhp_currentvalue _output_get)
      (set `/Game/Blueprint/Character/WBP_CharacterUIBase.MaxPosture` _maxposturepoint_currentvalue _output_get)
      (`self.ApplyHpToWidgetOnChanged`))
    (:`then_1`
      (`Widget.SetVisibility` (`WidgetComponent.GetWidget` (`self.CanShinobiDeathblowUIPos`)) "Hidden"))))

(fn `Parried`
  (params (Impact :type "Float (single-precision)"))
  (returns (ReturnValue :type Boolean))
  (bind (_posturepoint_basevalue _posturepoint_currentvalue) (break `GameplayAttributeData` (`CharacterAttributeSet.PosturePoint` (`self.CharacterAttributeSet`))))
  (`self.ParriedPlayMontage`)
  (`AbilitySystemComponent.BP_ApplyGameplayEffectToSelf` :`self` (`self.AbilitySystemComponent`) :`GameplayEffectClass` "/Game/Blueprint/GAS/Enemy/GE_Parried.GE_Parried_C")
  (`self.ApplyHitGameplayEffect` 0.0 Impact)
  (return (<= _posturepoint_currentvalue 0.0)))

(fn `SetCollisionReference`
  (set `self.WeaponCollisionCapsule` (`self.WeaponCollision`)))

(fn `SetRotationToPlayer`
  (params (DeltaTime :type "Float (double-precision)"))
  (`self.SetRotationToTarget` (- (`self.K2_GetActorLocation` (`GameplayStatics.GetPlayerCharacter` 0)) (`self.K2_GetActorLocation`)) DeltaTime))

(fn `SetUIVisible`
  (bind _returnvalue (`WidgetComponent.GetWidget` (`self.LockOnUI`)))
  (bind _returnvalue_2 (`WidgetComponent.GetWidget` (`self.CanShinobiDeathblowUIPos`)))
  (`|ExecutionSequence`
    (:`then_0`
      (if (and (`GameplayTagAssetInterface.HasMatchingGameplayTag` (`self.AbilitySystemComponent`) (struct :`TagName` "Ability.State.BrokePosture")) (`|EnumInequality` (`self.CharacterState`) "Dead"))
        (`Widget.SetVisibility` _returnvalue_2 "Visible")
        (else
          (`Widget.SetVisibility` _returnvalue_2 "Hidden"))))
    (:`then_1`
      (if (`self.GetIsTargeting`)
        (`Widget.SetVisibility` _returnvalue "Visible")
        (else
          (`Widget.SetVisibility` _returnvalue "Hidden"))))))

(fn `TakenDeathblow`
  (params (PlayerActor :type "/Game/Blueprint/Character/Player/BP_Player Object Reference"))
  (returns (PlayAbility :type "GameplayAbility Class Reference"))
  (bind _returnvalue (`self.K2_GetActorLocation` PlayerActor))
  (bind _shinobideathblowdata (`self.ShinobiDeathblowData`))
  ;[1 1 1] todo 向きによって変える
  (if true
    (`self.K2_SetActorLocation` (+ _returnvalue (* (`self.GetActorForwardVector` PlayerActor) (`/Game/Blueprint/Character/Enemy/DA_ShinobiDeathblowData.FrontDistance` _shinobideathblowdata))) true)
    (`self.K2_SetActorRotation` (`KismetMathLibrary.FindLookAtRotation` (`self.K2_GetActorLocation`) _returnvalue))
    (`AbilitySystemComponent.TryActivateAbilityByClass` (`self.AbilitySystemComponent`) (`/Game/Blueprint/Character/Enemy/DA_ShinobiDeathblowData.FrontDeathblowedAbility` _shinobideathblowdata) true)
    (return (`/Game/Blueprint/Character/Enemy/DA_ShinobiDeathblowData.FrontDeathblowAbility` _shinobideathblowdata))))

(fn `UserConstructionScript`)