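; Base Gameplay Ability for one step of a character's combo attack.
; A first attack starts immediately, while later steps wait for a single gameplay event before starting.
; Each step applies GE_Attack to the owner, plays its montage and copies its AttackParam to the owning CharacterBase once the montage task starts.
; The ability ends when the montage completes, blends out, is interrupted or is cancelled.
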(event `self.K2_ActivateAbility`
  (if (not (`self.IsFirstAttack`))
    (`AbilityTask_WaitGameplayEvent.WaitGameplayEvent` (struct) null true
      (:`EventReceived`
        _)))
  (`self.BP_ApplyGameplayEffectToOwner` "/Game/Blueprint/GAS/GE/GE_Attack.GE_Attack_C")
  (`AbilityTask_PlayMontageAndWait.CreatePlayMontageAndWaitProxy` "None" (`self.Montage to Play`)
    (:`then`
      ;[1 1 1] 攻撃パラメーターのセット
      (bind _ascharacter_base (cast `CharacterBase` (`self.GetOwningActorFromActorInfo`)))
      (set `CharacterBase.CharacterAttackParam` (`self.AttackParam`) _ascharacter_base))
    (:`OnCompleted`
      (`self.K2_EndAbility` :!label _label))
    (:`OnBlendOut`
      (goto _label))
    (:`OnInterrupted`
      (goto _label))
    (:`OnCancelled`
      (goto _label))))