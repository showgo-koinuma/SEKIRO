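; Gameplay ability that performs a deathblow, playing a GhostSamurai execution montage on the owning PlayerCharacter.
; When the montage starts, it switches the capsule to IgnoreOnlyPawn collision, animates camera arm length and location, and schedules an arm reset.
; Completion, blend out, interruption or cancellation all end the ability and restore the Pawn collision profile.
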(event `self.K2_ActivateAbility`
  (`AbilityTask_PlayMontageAndWait.CreatePlayMontageAndWaitProxy` "None" "/Game/Animation/AnimationMontage/ShinobiDeathblow/GhostSamurai_Execution05_Montage.GhostSamurai_Execution05_Montage"
    (:`then`
      (bind _asplayer_character (cast `PlayerCharacter` (`self.GetOwningActorFromActorInfo`)))
      (bind _capsulecomponent (`Character.CapsuleComponent` _asplayer_character))
      (`PrimitiveComponent.SetCollisionProfileName` _capsulecomponent "IgnoreOnlyPawn" true)
      (`PlayerCharacter.SetArmLengthAnim` _asplayer_character 200.0 0.3)
      (`PlayerCharacter.SetArmLocationAnim` _asplayer_character (`PlayerCharacter.ArmDefaultLocation` _asplayer_character) 0.3)
      (`PlayerCharacter.StartResetArm` _asplayer_character 1.7))
    (:`OnCompleted`
      (`self.K2_EndAbility` :!label _label)
      (`PrimitiveComponent.SetCollisionProfileName` _capsulecomponent "Pawn" true))
    (:`OnBlendOut`
      (goto _label))
    (:`OnInterrupted`
      (goto _label))
    (:`OnCancelled`
      (goto _label))))